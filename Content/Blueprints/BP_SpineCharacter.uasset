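; BP_SpineCharacter is a Gameplay Ability System character with a stamina-costed combo attack, which initializes its BP_HUD on possession.
; BeginPlay sets attributes from a Config data table through set-by-caller effects, grants the attack ability and caches its cost spec.
; IA_Attack selects a montage by combo index, activates the ability and applies cost on success.
; Presses during attacks queue the next montage, which TryContinueCombo triggers or otherwise resets.
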(event `self.ReceiveBeginPlay`
  (`self.InitAttributeValues`)
  (`self.InitAttackAbility` (`self.AbilitySystemComponent`)))

(event `self.ReceivePossessed`
  (params (NewController :type "Controller Object Reference"))
  (bind _asplayer_controller (cast `PlayerController` NewController))
  (bind _asbp_hud (cast `/Game/Blueprints/BP_HUD` (`PlayerController.GetHUD` _asplayer_controller)))
  (`/Game/Blueprints/BP_HUD.InitHUD` _asbp_hud))

(event `self.ReceiveTick`
  (params (DeltaSeconds :type "Float (single-precision)")))

(event `EnhancedInput|/Game/ThirdPerson/Input/Actions/IA_Attack`
  (params (ActionValue :type Boolean) (ElapsedSeconds :type "Float (double-precision)") (TriggeredSeconds :type "Float (double-precision)") (InputAction :type "InputAction Object Reference" :default "/Game/ThirdPerson/Input/Actions/IA_Attack.IA_Attack"))
  (:`Started`
    (if (`self.bIsPerformingAttackAbility`) :!label _label
      (set `self.ComboIndex` (+ 1 (`self.ComboIndex`)))
      (set `self.bShouldContinueCombo` true)
      (else
        (set `self.bShouldContinueCombo` false)
        (set `self.bIsPerformingAttackAbility` true)
        (set `self.MontageToPlay` (`|GetArrayItem` (`/Game/Blueprints/Data/BP_SpineData.ComboMontages` (`self.Config`)) (`self.ComboIndex`)))
        (bind _returnvalue (`AbilitySystemComponent.TryActivateAbility` (`self.AbilitySystemComponent`) (`self.AttackAbility`) true))
        (if _returnvalue
          (`self.ApplyAbilityCost`))))))

(event `TryContinueCombo`
  (set `self.bIsPerformingAttackAbility` false)
  (if (`self.bShouldContinueCombo`)
    (goto _label)
    (else
      (set `self.ComboIndex` 0))))

(fn `ApplyAbilityCost`
  (`AbilitySystemComponent.BP_ApplyGameplayEffectSpecToSelf` (`self.AbilitySystemComponent`) (`self.AttackAbilityCostSpec`)))

(fn `ApplyMaxAttributeValues`
  (params (AttributeTag :type "GameplayTag Structure") (AttributeValue :type "Float (double-precision)") (AbilitySystemComponent :type "AbilitySystemComponent Object Reference"))
  (bind _returnvalue (`AbilitySystemBlueprintLibrary.AssignTagSetByCallerMagnitude` (`AbilitySystemComponent.MakeOutgoingSpec` :`self` AbilitySystemComponent :`GameplayEffectClass` "/Game/Blueprints/GameplayEffects/GE_ApplyMaxAttributes.GE_ApplyMaxAttributes_C" :`Level` 1.0) AttributeTag AttributeValue))
  (`AbilitySystemComponent.BP_ApplyGameplayEffectSpecToSelf` AbilitySystemComponent _returnvalue)
  (return))

(fn `ApplyStartingAttributeValues`
  (params (AbilitySystemComponent :type "AbilitySystemComponent Object Reference"))
  (`AbilitySystemComponent.BP_ApplyGameplayEffectToSelf` :`self` AbilitySystemComponent :`GameplayEffectClass` "/Game/Blueprints/GameplayEffects/GE_ApplyStartingAttributes.GE_ApplyStartingAttributes_C" :`Level` 1.0))

(fn `InitAttackAbility`
  (params (AbilitySysytemComponent :type "AbilitySystemComponent Object Reference"))
  (bind (_attackability_ability _attackability_cost) (break `/Game/Blueprints/Struct/S_StartingAbility` (`/Game/Blueprints/Data/BP_SpineData.AttackAbility` (`self.Config`))))
  (bind _returnvalue (`AbilitySystemComponent.K2_GiveAbility` AbilitySysytemComponent _attackability_ability 1 -1))
  (set `self.AttackAbility` _returnvalue)
  (bind _returnvalue_2 (`AbilitySystemBlueprintLibrary.AssignTagSetByCallerMagnitude` (`AbilitySystemComponent.MakeOutgoingSpec` :`self` AbilitySysytemComponent :`GameplayEffectClass` "/Game/Blueprints/GameplayEffects/GE_StaminaCost.GE_StaminaCost_C" :`Level` 1.0) (struct :`TagName` "Attribute.Stamina") (* _attackability_cost -1.0)))
  (set `self.AttackAbilityCostSpec` _returnvalue_2))

(fn `InitAttributes`)

(fn `InitAttributeValues`
  (bind _returnvalue (`|GetDataTableRow` (`/Game/Blueprints/Data/BP_SpineData.InitialAttributesDataTable` (`self.Config`)) "Default")
    (:`then`
      (bind (_maxhealth _maxstamina) (break `SpineAttributeRow` _returnvalue))
      (`self.ApplyMaxAttributeValues` (struct :`TagName` "Attribute.MaxHealth") _maxhealth (`self.AbilitySystemComponent`))
      (`self.ApplyMaxAttributeValues` (struct :`TagName` "Attribute.MaxStamina") _maxstamina (`self.AbilitySystemComponent`))
      (`self.ApplyStartingAttributeValues` (`self.AbilitySystemComponent`)))))

(fn `UserConstructionScript`)